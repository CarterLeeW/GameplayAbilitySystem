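; Arcane Shards ability that shows a magic circle, then on input press casts a level-scaled burst of shards at the targeted ground point.
; A spawned BP_PointCollection supplies randomly rotated ground points while the avatar motion-warps to face the target.
; A montage event starts a looping timer that, per point, applies radial damage to nearby live players except the caster and fires a GameplayCue.
; Once all shards spawn, it cleans up and ends.
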(event `self.K2_ActivateAbility`
  (`|ExecutionSequence`
    (:`then_0`
      (message `PlayerInterface.ShowMagicCircle` (`self.GetAvatarActorFromActorInfo`) null))
    (:`then_1`
      (`AbilityTask_WaitInputPress.WaitInputPress` false
        (:`OnPress`
          (bind (_asynctaskproxy _datahandle) (`TargetDataUnderMouse.CreateTargetDataUnderMouse`)
            (:`ValidData`
              (`|ExecutionSequence`
                (:`then_0`
                  (bind (_bblockinghit _binitialoverlap _time _distance _location _impactpoint) (`GameplayStatics.BreakHitResult` (`AbilitySystemBlueprintLibrary.GetHitResultFromTargetData` _datahandle)))
                  (message `CombatInterface.UpdateWarpFacingTarget` (`self.GetAvatarActorFromActorInfo`) _impactpoint)
                  (bind _returnvalue (`|SpawnActorFromClass` "/Game/Blueprints/AbilitySystem/Aura/Ability/Arcane/ArcaneShards/BP_PointCollection.BP_PointCollection_C" (`KismetMathLibrary.Conv_VectorToTransform` _impactpoint) "AlwaysSpawn" "MultiplyWithRoot" null null))
                  (set `self.PointCollection` _returnvalue)
                  (set `self.GroundPoints` (`PointCollection.GetGroundPoints` (`self.PointCollection`) _impactpoint (`AuraAbilitySystemLibrary.GetValueAtLevel_Int32` (`self.GetAbilityLevel`) (`self.NumShards`)) (`KismetMathLibrary.RandomFloatInRange` 0.0 360.0)))
                  (message `PlayerInterface.HideMagicCircle` (`self.GetAvatarActorFromActorInfo`)))
                (:`then_1`
                  (`AbilityTask_PlayMontageAndWait.CreatePlayMontageAndWaitProxy` "None" "/Game/Assets/Characters/Aura/Animations/Abilities/AM_Cast_ArcaneShards.AM_Cast_ArcaneShards" 1.0 "None" false
                    (:`then`
                      (`AbilityTask_WaitGameplayEvent.WaitGameplayEvent` (struct :`TagName` "Event.Montage.ArcaneShards") null true
                        (:`EventReceived`
                          (bind _returnvalue_2 (`KismetSystemLibrary.K2_SetTimerDelegate` (delegate `SpawnShard`) (`self.ShardSpawnInterval`) true))
                          (set `self.ShardSpawnTimer` _returnvalue_2)
                          (`self.SpawnShard`))))
                    (:`OnInterrupted`
                      (`self.K2_EndAbility` :!label _label))
                    (:`OnCancelled`
                      (goto _label))))))))))))

(event `SpawnShard`
  (if (< (`self.ShardCount`) (`AuraAbilitySystemLibrary.GetValueAtLevel_Int32` (`self.GetAbilityLevel`) (`self.NumShards`)))
    (`self.SpawnShardsLoop`)
    (else
      (`self.DestroyAndClearVariables`)
      (`KismetSystemLibrary.Delay` 0.2)
      (`self.K2_EndAbility`))))

(fn `DestroyAndClearVariables`
  (`Actor.K2_DestroyActor` (`self.PointCollection`))
  (set `self.GroundPoints` (`|MakeArray` null :!type "SceneComponent Object Reference"))
  (`KismetSystemLibrary.K2_ClearAndInvalidateTimerHandle` (`self.ShardSpawnTimer`))
  (set `self.ShardCount` 0))

(fn `SpawnShardsLoop`
  (locals (ShardSpawnLocation :type "Vector Structure" :default (0.0 0.0 0.0)) (OverlappingPlayers :type "Array of Actor Object Reference"))
  (set `local.ShardSpawnLocation` (`SceneComponent.K2_GetComponentLocation` (`|GetArrayItem` (`self.GroundPoints`) (`self.ShardCount`))))
  (bind _outoverlappingactors (`AuraAbilitySystemLibrary.GetLivePlayersWithinRadius` (`|MakeArray` (`self.GetAvatarActorFromActorInfo`)) (`self.RadialDamageOuterRadius`) (`local.ShardSpawnLocation`)))
  (bind _output_get (set `local.OverlappingPlayers` _outoverlappingactors))
  (for _array_element _output_get
    (bind _structout (setmembers `DamageEffectParams` :`StructRef` (`self.MakeDamageEffectParamsFromClassDefaults` _array_element) :`RadialDamageOrigin` (`local.ShardSpawnLocation`)))
    (`AuraAbilitySystemLibrary.ApplyDamageEffect` _structout))
  (`self.K2_ExecuteGameplayCueWithParams` (struct :`TagName` "GameplayCue.ArcaneShards") (`AbilitySystemBlueprintLibrary.MakeGameplayCueParameters` 0.0 0.0 (struct) (struct) (struct) (struct) (struct) (`local.ShardSpawnLocation`)))
  (`/Engine/EditorBlueprintResources/StandardMacros.IncrementInt` (`self.ShardCount`)))