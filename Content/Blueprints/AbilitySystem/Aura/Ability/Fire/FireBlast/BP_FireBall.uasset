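; BP_FireBall is the fireball projectile for the Fire Blast ability, which flies out and then returns to its owner.
; After a delay from BeginPlay, it turns on homing toward the owner's root component and flags itself as returning.
; SpawnExplosionEffects executes the FireBall impact gameplay cue on the owner, passing the fireball's location so effects run through the Gameplay Cue system.
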(event `self.ReceiveBeginPlay`
  (`KismetSystemLibrary.Delay` (`self.SecondsBeforeReturning`))
  (`/Engine/EditorBlueprintResources/StandardMacros.IsValid` (`self.GetOwner`)
    (:`Is Valid`
      (set `ProjectileMovementComponent.bIsHomingProjectile` true (`self.ProjectileMovement`))
      (set `ProjectileMovementComponent.HomingTargetComponent` (`Actor.RootComponent` (`self.GetOwner`)) (`self.ProjectileMovement`))
      (set `self.bIsReturning` true))))

(event `self.SpawnExplosionEffects`
  (bind _returnvalue (`self.GetOwner`))
  (`/Engine/EditorBlueprintResources/StandardMacros.IsValid` _returnvalue
    (:`Is Valid`
      (`GameplayCueFunctionLibrary.ExecuteGameplayCueOnActor` _returnvalue (struct :`TagName` "GameplayCue.FireBall.ImpactEffects") (`AbilitySystemBlueprintLibrary.MakeGameplayCueParameters` 0.0 0.0 (struct) (struct) (struct) (struct) (struct) (`self.K2_GetActorLocation`))))))

(event `self.ReceiveTick`
  (params (DeltaSeconds :type "Float (single-precision)")))

(fn `UserConstructionScript`)