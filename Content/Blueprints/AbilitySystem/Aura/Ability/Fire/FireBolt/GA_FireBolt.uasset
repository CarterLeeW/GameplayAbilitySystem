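; GA_FireBolt is a gameplay ability that casts a Fire Bolt projectile at the location under the mouse.
; On activation, it takes the cursor hit location from target data and sends it to the avatar as a warp facing target.
; It then plays the cast montage, spawns the projectile toward that location when the montage's gameplay event arrives, and ends when the montage completes.
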(event `self.K2_ActivateAbility`
  (bind (_asynctaskproxy _datahandle) (`TargetDataUnderMouse.CreateTargetDataUnderMouse`)
    (:`ValidData`
      (bind _output_get (set `self.Projectile Target Location` (`.Location` (`GameplayStatics.BreakHitResult` (`AbilitySystemBlueprintLibrary.GetHitResultFromTargetData` _datahandle)))))
      (message `CombatInterface.UpdateWarpFacingTarget` (`self.GetAvatarActorFromActorInfo`) _output_get)
      (`AbilityTask_PlayMontageAndWait.CreatePlayMontageAndWaitProxy` "None" "/Game/Assets/Characters/Aura/Animations/Abilities/AM_Cast_FireBolt.AM_Cast_FireBolt"
        (:`then`
          (`AbilityTask_WaitGameplayEvent.WaitGameplayEvent` (struct :`TagName` "Event.Montage.FireBolt") null
            (:`EventReceived`
              (`self.SpawnProjectileSpell` (`self.Projectile Target Location`)))))
        (:`OnCompleted`
          (`self.K2_EndAbility`))))))