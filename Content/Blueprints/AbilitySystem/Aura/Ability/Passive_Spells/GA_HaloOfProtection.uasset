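; GA_HaloOfProtection is a passive gameplay ability that boosts the owner's Arcane, Fire, Lightning and Physical resistances while active.
; On activation it turns the level-scaled PercentOfDamageDeflected into a multiplier and passes it to a GE_HaloOfProtection spec through Set By Caller resistance tags.
; It applies that spec to itself and stores the active effect handle, which it uses to remove the effect when the ability ends.
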(event `self.K2_ActivateAbility`
  (bind _returnvalue (`self.GetAbilitySystemComponentFromActorInfo`))
  (set `self.SpecHandle` (`AbilitySystemComponent.MakeOutgoingSpec` _returnvalue "/Game/Blueprints/AbilitySystem/Aura/Ability/Passive_Spells/GE_HaloOfProtection.GE_HaloOfProtection_C" (`KismetMathLibrary.Conv_IntToDouble` (`self.GetAbilityLevel`)) (`AbilitySystemComponent.MakeEffectContext` _returnvalue)))
  (set `self.ResistanceMultiplier` (+ (/ (`AuraAbilitySystemLibrary.GetValueAtLevel_Float` (`self.GetAbilityLevel`) (`self.PercentOfDamageDeflected`)) 100.0) 1.0))
  (`|ExecutionSequence`
    (:`then_0`
      (`AbilitySystemBlueprintLibrary.AssignTagSetByCallerMagnitude` (`self.SpecHandle`) (struct :`TagName` "Attributes.Resistance.Arcane") (`self.ResistanceMultiplier`)))
    (:`then_1`
      (`AbilitySystemBlueprintLibrary.AssignTagSetByCallerMagnitude` (`self.SpecHandle`) (struct :`TagName` "Attributes.Resistance.Fire") (`self.ResistanceMultiplier`)))
    (:`then_2`
      (`AbilitySystemBlueprintLibrary.AssignTagSetByCallerMagnitude` (`self.SpecHandle`) (struct :`TagName` "Attributes.Resistance.Lightning") (`self.ResistanceMultiplier`)))
    (:`then_3`
      (`AbilitySystemBlueprintLibrary.AssignTagSetByCallerMagnitude` (`self.SpecHandle`) (struct :`TagName` "Attributes.Resistance.Physical") (`self.ResistanceMultiplier`)))
    (:`then_4`
      (bind _returnvalue_2 (`AbilitySystemComponent.BP_ApplyGameplayEffectSpecToSelf` (`self.GetAbilitySystemComponentFromActorInfo`) (`self.SpecHandle`)))
      (set `self.ActiveGameplayEffect` _returnvalue_2))))

(event `self.K2_OnEndAbility`
  (params (bWasCancelled :type Boolean))
  (`AbilitySystemComponent.RemoveActiveGameplayEffect` (`self.GetAbilitySystemComponentFromActorInfo`) (`self.ActiveGameplayEffect`) -1))