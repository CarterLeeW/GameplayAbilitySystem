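; GA_LifeSiphon is a passive gameplay ability that restores health to its owner when an actor death event arrives.
; On activation it waits for the Event.ActorDeath gameplay event.
; Each event builds a GE_LifeSiphon spec at ability level and applies it to the owner.
; The heal is a level-scaled percentage of the avatar's max health, passed as a SetByCaller magnitude on the health tag.
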(event `self.K2_ActivateAbility`
  (bind _returnvalue (`self.GetAbilitySystemComponentFromActorInfo`))
  (`AbilityTask_WaitGameplayEvent.WaitGameplayEvent` (struct :`TagName` "Event.ActorDeath") null
    (:`EventReceived`
      (set `self.SpecHandle` (`AbilitySystemComponent.MakeOutgoingSpec` _returnvalue "/Game/Blueprints/AbilitySystem/Aura/Ability/Passive_Spells/GE_LifeSiphon.GE_LifeSiphon_C" (`KismetMathLibrary.Conv_IntToDouble` (`self.GetAbilityLevel`)) (`AbilitySystemComponent.MakeEffectContext` _returnvalue)))
      (bind _returnvalue_2 (message `CombatInterface.GetMaxHealthValue` (`self.GetAvatarActorFromActorInfo`)))
      (`AbilitySystemBlueprintLibrary.AssignTagSetByCallerMagnitude` (`self.SpecHandle`) (struct :`TagName` "Attributes.Vital.Health") (* _returnvalue_2 (/ (`AuraAbilitySystemLibrary.GetValueAtLevel_Float` (`self.GetAbilityLevel`) (`self.PercentOfHealthRestored`)) 100.0)))
      (`AbilitySystemComponent.BP_ApplyGameplayEffectSpecToSelf` (`self.GetAbilitySystemComponentFromActorInfo`) (`self.SpecHandle`)))))

(event `self.K2_OnEndAbility`
  (params (bWasCancelled :type Boolean)))