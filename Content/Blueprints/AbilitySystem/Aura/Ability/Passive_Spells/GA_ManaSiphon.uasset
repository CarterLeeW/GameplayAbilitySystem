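; GA_ManaSiphon is a passive gameplay ability meant to restore a percentage of the avatar's max mana on actor death.
; On each Event.ActorDeath gameplay event, it applies a GE_ManaSiphon spec to itself with a set-by-caller mana magnitude.
; The level-scaled PercentOfManaRestored drives that magnitude, but it multiplies 0.0 here, as the fetched max mana is not shown feeding it.
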(event `self.K2_ActivateAbility`
  (bind _returnvalue (`self.GetAbilitySystemComponentFromActorInfo`))
  (`AbilityTask_WaitGameplayEvent.WaitGameplayEvent` (struct :`TagName` "Event.ActorDeath") null
    (:`EventReceived`
      (set `self.SpecHandle` (`AbilitySystemComponent.MakeOutgoingSpec` _returnvalue "/Game/Blueprints/AbilitySystem/Aura/Ability/Passive_Spells/GE_ManaSiphon.GE_ManaSiphon_C" (`KismetMathLibrary.Conv_IntToDouble` (`self.GetAbilityLevel`)) (`AbilitySystemComponent.MakeEffectContext` _returnvalue)))
      (message `CombatInterface.GetMaxManaValue` (`self.GetAvatarActorFromActorInfo`))
      (`AbilitySystemBlueprintLibrary.AssignTagSetByCallerMagnitude` (`self.SpecHandle`) (struct :`TagName` "Attributes.Vital.Mana") (* 0.0 (/ (`AuraAbilitySystemLibrary.GetValueAtLevel_Float` (`self.GetAbilityLevel`) (`self.PercentOfManaRestored`)) 100.0)))
      (`AbilitySystemComponent.BP_ApplyGameplayEffectSpecToSelf` (`self.GetAbilitySystemComponentFromActorInfo`) (`self.SpecHandle`)))))

(event `self.K2_OnEndAbility`
  (params (bWasCancelled :type Boolean)))