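; GA_MeleeAttack is an enemy gameplay ability that performs a melee attack against the avatar's combat target.
; It updates motion-warp facing toward the target and plays a random tagged attack montage.
; When the montage's gameplay event fires, it finds live players around that attack's combat socket, draws a debug sphere there, and damages non-friends.
; The ability ends when the montage completes, is interrupted or cancelled.
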(event `self.K2_ActivateAbility`
  (bind _returnvalue (`self.GetAvatarActorFromActorInfo`))
  (bind _returnvalue_2 (`self.GetAvatarActorFromActorInfo`))
  (bind _returnvalue_3 (message `EnemyInterface.GetCombatTarget` _returnvalue))
  (bind _ascombat_interface (cast `CombatInterface` _returnvalue)
    (:`then`
      (`CombatInterface.UpdateWarpFacingTarget` _ascombat_interface (`Actor.K2_GetActorLocation` _returnvalue_3))
      (bind _returnvalue_4 (message `CombatInterface.GetAttackMontages` _returnvalue))
      (bind _output_get (set `self.TaggedMontageToUse` (`KismetArrayLibrary.Array_Random` _returnvalue_4)))
      (bind (_montage _montagetag) (break `TaggedMontage` _output_get))
      (`AbilityTask_PlayMontageAndWait.CreatePlayMontageAndWaitProxy` "None" _montage
        (:`then`
          (`AbilityTask_WaitGameplayEvent.WaitGameplayEvent` _montagetag null
            (:`EventReceived`
              (bind _returnvalue_5 (message `CombatInterface.GetCombatSocketLocation` _returnvalue_2 _montagetag))
              (`KismetSystemLibrary.DrawDebugSphere` _returnvalue_5 45.0 12 (struct :`R` 1.0 :`G` 1.0 :`B` 1.0 :`A` 1.0) 1.0)
              (bind _outoverlappingactors (`AuraAbilitySystemLibrary.GetLivePlayersWithinRadius` (`|MakeArray` _returnvalue_2) 70.0 _returnvalue_5))
              (for _array_element _outoverlappingactors
                (if (`AuraAbilitySystemLibrary.IsNotFriend` (`self.GetAvatarActorFromActorInfo`) _array_element)
                  (`self.CauseDamage` _array_element))))))
        (:`OnCompleted`
          (`self.K2_EndAbility` :!label _label))
        (:`OnInterrupted`
          (goto _label))
        (:`OnCancelled`
          (goto _label))))
    (:`CastFailed`
      (`self.K2_EndAbility`))))