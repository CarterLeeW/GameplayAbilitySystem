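; Enemy ranged attack gameplay ability that launches a projectile at the avatar's current combat target.
; On activation it turns the avatar toward the target through the combat interface's warp facing, then plays a random tagged attack montage.
; The montage's gameplay event triggers a projectile spawn from that montage's socket, aimed at the target's location at that moment.
; The ability ends when the montage completes, is interrupted or cancelled, or the interface cast fails.
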(event `self.K2_ActivateAbility`
  (bind _returnvalue (`self.GetAvatarActorFromActorInfo`))
  (bind (_tagged_montage_to_use_montage _tagged_montage_to_use_montagetag _tagged_montage_to_use_sockettag) (break `TaggedMontage` (`self.Tagged Montage to Use`)))
  (bind _tagged_montage_to_use_montage_2 (break `TaggedMontage` (`self.Tagged Montage to Use`)))
  (bind (_tagged_montage_to_use_montage_3 _tagged_montage_to_use_montagetag_2) (break `TaggedMontage` (`self.Tagged Montage to Use`)))
  (bind _returnvalue_2 (message `EnemyInterface.GetCombatTarget` _returnvalue))
  (bind _ascombat_interface (cast `CombatInterface` _returnvalue)
    (:`then`
      (`CombatInterface.UpdateWarpFacingTarget` _ascombat_interface (`Actor.K2_GetActorLocation` _returnvalue_2))
      (bind _returnvalue_3 (message `CombatInterface.GetAttackMontages` _returnvalue))
      (set `self.Tagged Montage to Use` (`KismetArrayLibrary.Array_Random` _returnvalue_3))
      (`AbilityTask_PlayMontageAndWait.CreatePlayMontageAndWaitProxy` "None" _tagged_montage_to_use_montage_2
        (:`then`
          (`AbilityTask_WaitGameplayEvent.WaitGameplayEvent` _tagged_montage_to_use_montagetag_2 null
            (:`EventReceived`
              (bind _returnvalue_4 (message `EnemyInterface.GetCombatTarget` (`self.GetAvatarActorFromActorInfo`)))
              (`self.SpawnProjectileSpell` (`Actor.K2_GetActorLocation` _returnvalue_4) _tagged_montage_to_use_sockettag))))
        (:`OnCompleted`
          (`self.K2_EndAbility` :!label _label))
        (:`OnInterrupted`
          (goto _label))
        (:`OnCancelled`
          (goto _label))))
    (:`CastFailed`
      (`self.K2_EndAbility`))))