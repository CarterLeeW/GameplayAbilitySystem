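; Melee attack gameplay ability that plays an avatar's attack montage and damages nearby live players.
; On activation it updates the motion-warp facing toward the combat target through CombatInterface, then plays a randomly picked tagged montage.
; The montage's gameplay event triggers a small radius query at the matching combat socket, causing damage to each player found except the avatar.
; The ability ends when the montage completes or the interface cast fails.
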(event `self.K2_ActivateAbility`
  (bind _returnvalue (`self.GetAvatarActorFromActorInfo`))
  (bind _returnvalue_2 (`self.GetAvatarActorFromActorInfo`))
  (bind _returnvalue_3 (message `EnemyInterface.GetCombatTarget` _returnvalue))
  (bind _ascombat_interface (cast `CombatInterface` _returnvalue)
    (:`then`
      (`CombatInterface.UpdateWarpFacingTarget` _ascombat_interface (`Actor.K2_GetActorLocation` _returnvalue_3))
      (bind _returnvalue_4 (message `CombatInterface.GetAttackMontages` _returnvalue))
      (bind (_montage _montagetag) (break `TaggedMontage` (`KismetArrayLibrary.Array_Random` _returnvalue_4)))
      (`AbilityTask_PlayMontageAndWait.CreatePlayMontageAndWaitProxy` "None" _montage
        (:`then`
          (`AbilityTask_WaitGameplayEvent.WaitGameplayEvent` _montagetag null
            (:`EventReceived`
              (bind _returnvalue_5 (message `CombatInterface.GetCombatSocketLocation` _returnvalue_2 _montagetag))
              (bind _outoverlappingactors (`AuraAbilitySystemLibrary.GetLivePlayersWithinRadius` (`|MakeArray` _returnvalue_2) 45.0 _returnvalue_5))
              (for _array_element _outoverlappingactors
                (`self.CauseDamage` _array_element)))))
        (:`OnCompleted`
          (`self.K2_EndAbility`))))
    (:`CastFailed`
      (`self.K2_EndAbility`))))