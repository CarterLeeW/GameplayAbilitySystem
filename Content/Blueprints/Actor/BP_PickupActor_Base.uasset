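; Base pickup actor with a mesh and a sphere collision that reacts when another actor overlaps it.
; On BeginPlay it caches the mesh's original scale, then plays a timeline whose scale track uniformly multiplies that scale to animate the mesh.
; The sphere's begin-overlap event forwards the other actor to OnOverlap, which has no logic in this graph.
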(event `self.ReceiveBeginPlay`
  ;[1 1 1] Better way to implement this for loot items??
  (set `self.MeshOriginalScale` (`SceneComponent.RelativeScale3D` (`self.Mesh`)))
  (bind (_direction _scaletrack) (`Timeline|Timeline`)
    (:`Update`
      (`SceneComponent.SetRelativeScale3D` (`self.Mesh`) (* (`self.MeshOriginalScale`) (`KismetMathLibrary.MakeVector` _scaletrack _scaletrack _scaletrack))))))

(event `self.SphereCollision.OnComponentBeginOverlap`
  (params (OverlappedComponent :type "PrimitiveComponent Object Reference") (OtherActor :type "Actor Object Reference") (OtherComp :type "PrimitiveComponent Object Reference") (OtherBodyIndex :type Integer) (bFromSweep :type Boolean) (SweepResult :type "HitResult Structure (by ref)"))
  (`self.OnOverlap` OtherActor))

(fn `UserConstructionScript`)