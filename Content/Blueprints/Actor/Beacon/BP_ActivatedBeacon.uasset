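; Beacon actor that lights up when an actor implementing PlayerInterface enters its sphere.
; The overlap sets Reached, runs BeaconActivated, then fires the Activated dispatcher and unbinds its listeners.
; Activation runs once, guarded by the dynamic material's validity: it disables sphere collision and plays a timeline driving the mesh's Glow parameter.
; LoadActor replays activation for reached beacons without broadcasting.
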(event `BeaconActivated`
  (`self.GlowMaterialDynamic`
    (:`then`)
    (:`else`
      (`PrimitiveComponent.SetCollisionEnabled` (`self.Sphere`) "NoCollision")
      (bind _returnvalue (`KismetMaterialLibrary.CreateDynamicMaterialInstance` (`PrimitiveComponent.GetMaterial` (`self.Mesh`) 0)))
      (bind _output_get (set `self.GlowMaterialDynamic` _returnvalue))
      (`PrimitiveComponent.SetMaterial` (`self.Mesh`) 0 _output_get)
      (bind (_direction _glowtrack) (`Timeline|GlowTimeline`)
        (:`Update`
          (`MaterialInstanceDynamic.SetScalarParameterValue` (`self.GlowMaterialDynamic`) "Glow" (* _glowtrack (`self.GlowConstant`))))))))

(event `self.Sphere.OnComponentBeginOverlap`
  (params (OverlappedComponent :type "PrimitiveComponent Object Reference") (OtherActor :type "Actor Object Reference") (OtherComp :type "PrimitiveComponent Object Reference") (OtherBodyIndex :type Integer) (bFromSweep :type Boolean) (SweepResult :type "HitResult Structure (by ref)"))
  (if (`KismetSystemLibrary.DoesImplementInterface` OtherActor "/Script/Aura.PlayerInterface")
    (set `self.bReached` true)
    (`self.BeaconActivated`)
    (`self.Activated`)
    (clear `self.Activated`)))

(event `SaveObjectInterface.LoadActor`
  (if (`self.bReached`)
    (`self.BeaconActivated`)))

(fn `UserConstructionScript`)