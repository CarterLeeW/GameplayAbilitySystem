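; Oval brazier with three flames, each lit by a linked activated beacon, that opens a linked gate once all three burn.
; Beacon events turn on the matching particle and point light, set its flag, and recheck the gate, which triggers only once.
; Flame 0 also runs an intensity fade timeline, which leads into randomly chained flicker timelines scaling all three lights.
; LoadActor replays activation from the flame flags to restore state.
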(event `GateActivated`
  ;[1 1 1] Only activate once
  (if (not (`self.bGateActivated`))
    (set `self.bGateActivated` true)
    (bind _bp_activatedgate (`self.BP_ActivatedGate`)
      (:`then`
        (`/Game/Blueprints/Actor/Gate/BP_ActivatedGate.Open` _bp_activatedgate))
      (:`else`))))

(event `Beacon2Activated`
  ;[1 1 1] Bind Activation Events for Activated Beacons
  (`self.BeaconActivated_2`))

(event `Beacon0Activated`
  ;[1 1 1] Bind Activation Events for Activated Beacons
  (`self.BeaconActivated_0`))

(event `Beacon1Activated`
  ;[1 1 1] Bind Activation Events for Activated Beacons
  (`self.BeaconActivated_1`))

(event `self.ReceiveBeginPlay`
  (`|ExecutionSequence`
    (:`then_0`
      ;[1 1 1] Cast to Activated Beacons
      (bind _asbp_activated_beacon (cast `/Game/Blueprints/Actor/Beacon/BP_ActivatedBeacon` (`self.Trigger_0`)))
      (set `self.BP_ActivatedBeacon_0` _asbp_activated_beacon)
      (bind _asbp_activated_beacon_2 (cast `/Game/Blueprints/Actor/Beacon/BP_ActivatedBeacon` (`self.Trigger_1`)))
      (set `self.BP_ActivatedBeacon_1` _asbp_activated_beacon_2)
      (bind _asbp_activated_beacon_3 (cast `/Game/Blueprints/Actor/Beacon/BP_ActivatedBeacon` (`self.Trigger_2`)))
      (set `self.BP_ActivatedBeacon_2` _asbp_activated_beacon_3))
    (:`then_1`
      ;[1 1 1] Bind Activation Events for Activated Beacons
      (add `/Game/Blueprints/Actor/Beacon/BP_ActivatedBeacon.Activated` (`self.BP_ActivatedBeacon_0`) (delegate `Beacon0Activated`))
      (add `/Game/Blueprints/Actor/Beacon/BP_ActivatedBeacon.Activated` (`self.BP_ActivatedBeacon_1`) (delegate `Beacon1Activated`))
      (add `/Game/Blueprints/Actor/Beacon/BP_ActivatedBeacon.Activated` (`self.BP_ActivatedBeacon_2`) (delegate `Beacon2Activated`)))
    (:`then_2`
      ;[1 1 1] Cast to Activated Gate
      (bind _asbp_activated_gate (cast `/Game/Blueprints/Actor/Gate/BP_ActivatedGate` (`self.GateToOpen`)))
      (set `self.BP_ActivatedGate` _asbp_activated_gate))))

(event `SaveObjectInterface.LoadActor`
  ;[1 1 1] Load Actor and check if flames should be activated
  (`|ExecutionSequence`
    (:`then_0`
      (if (`self.bFlame_0_On`)
        (`self.BeaconActivated_0`)))
    (:`then_1`
      (if (`self.bFlame_1_On`)
        (`self.BeaconActivated_1`)))
    (:`then_2`
      (if (`self.bFlame_2_On`)
        (`self.BeaconActivated_2`)))))

(event `ChooseTimeline`
  ;[1 1 1] Flicker Randomization
  (switch `int` (`KismetMathLibrary.RandomIntegerInRange` 0 1)
    (:`Default`
      (`self.StartTimeline_1` :!label _label))
    (:`0`
      (`self.StartTimeline_0`))
    (:`1`
      (goto _label))))

(event `FlameOn_0`
  ;[1 1 1] Flame Activation
  (bind (_direction _intensity) (`Timeline|FlameActivate_0` :!via `PlayFromStart`)
    (:`Update`
      (`LightComponent.SetIntensity` (`self.PointLight_0`) (* _intensity (`self.BaseIntensity`))))
    (:`Finished`
      (`self.ChooseTimeline`))))

(event `StartTimeline_1`
  ;[1 1 1] Flame Flicker
  (bind (_direction _flameintensity) (`Timeline|FlameIntensity_1` :!via `PlayFromStart`)
    (:`Update`
      (`self.ScaleFlameIntensity_All` _flameintensity))
    (:`Finished`
      (`self.ChooseTimeline`))))

(event `FlameOn_1`
  ;[1 1 1] Flame Activation
  (bind (_direction _intensity) (`Timeline|FlameActivate_1` :!via `PlayFromStart`)
    (:`Update`
      (`LightComponent.SetIntensity` (`self.PointLight_1`) (* _intensity (`self.BaseIntensity`))))
    (:`Finished`
      (`self.ChooseTimeline`))))

(event `StartTimeline_0`
  ;[1 1 1] Flame Flicker
  (bind (_direction _flameintensity) (`Timeline|FlameIntensity_0` :!via `PlayFromStart`)
    (:`Update`
      (`self.ScaleFlameIntensity_All` _flameintensity))
    (:`Finished`
      (`self.ChooseTimeline`))))

(event `FlameOn_2`
  ;[1 1 1] Flame Activation
  (bind (_direction _intensity) (`Timeline|FlameActivate_2` :!via `PlayFromStart`)
    (:`Update`
      (`LightComponent.SetIntensity` (`self.PointLight_2`) (* _intensity (`self.BaseIntensity`))))
    (:`Finished`
      (`self.ChooseTimeline`))))

(fn `ActivateFlame_0`
  (`ActorComponent.Activate` (`self.Flame_0`) false)
  (`SceneComponent.SetVisibility` (`self.PointLight_0`) true false)
  (`self.FlameOn_0`))

(fn `BeaconActivated_0`
  (`ActorComponent.Activate` (`self.Flame_0`) false)
  (`SceneComponent.SetVisibility` (`self.PointLight_0`) true false)
  (`self.FlameOn_0`)
  (set `self.bFlame_0_On` true)
  (`self.Update Gate Activation`))

(fn `BeaconActivated_1`
  (`ActorComponent.Activate` (`self.Flame_1`) false)
  (`SceneComponent.SetVisibility` (`self.PointLight_1`) true false)
  (set `self.bFlame_1_On` true)
  (`self.Update Gate Activation`))

(fn `BeaconActivated_2`
  (`ActorComponent.Activate` (`self.Flame_2`) false)
  (`SceneComponent.SetVisibility` (`self.PointLight_2`) true false)
  (set `self.bFlame_2_On` true)
  (`self.Update Gate Activation`))

(fn `ScaleFlameIntensity_All`
  (params (Scale :type "Float (double-precision)"))
  (`LightComponent.SetIntensity` (`self.PointLight_0`) (* Scale (`self.BaseIntensity`)))
  (`LightComponent.SetIntensity` (`self.PointLight_1`) (* Scale (`self.BaseIntensity`)))
  (`LightComponent.SetIntensity` (`self.PointLight_2`) (* Scale (`self.BaseIntensity`))))

(fn `Update Gate Activation`
  ;[1 1 1] Just check for truth, bGateActivated is set in GateActivated event
  (if (and (`self.bFlame_0_On`) (`self.bFlame_1_On`) (`self.bFlame_2_On`))
    (`self.GateActivated`)))

(fn `UserConstructionScript`)