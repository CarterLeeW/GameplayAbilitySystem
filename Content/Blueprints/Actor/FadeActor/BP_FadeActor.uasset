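; Actor that fades its mesh out and back in, ignoring a custom cursor-visibility trace channel while faded.
; Construction caches original materials and collision response, and builds dynamic instances from designated fade materials.
; FadeOut swaps these in and a timeline drives their Fade parameter; FadeIn reverses it, resetting materials and collision once Fade completes at full value.
; BeginPlay runs a delayed fade-out then fade-in automatically.
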(event `FadeOut`
  (`PrimitiveComponent.SetCollisionResponseToChannel` (`self.Mesh`) "ECC_GameTraceChannel2" "ECR_Ignore")
  (`self.SetMaterialsToDynamicInstances`)
  (bind (_direction _fade) (`Timeline|Fade` :!label _label)
    (:`Update`
      (for _array_element (`self.DynamicMaterialInstances`)
        (`MaterialInstanceDynamic.SetScalarParameterValue` _array_element "Fade" _fade)))
    (:`Finished`
      (if (>= _fade 1.0)
        (`self.ResetMaterials`)
        (`PrimitiveComponent.SetCollisionResponseToChannel` (`self.Mesh`) "ECC_GameTraceChannel2" (`self.OriginalCursorVisResponse`))))))

(event `FadeIn`
  (goto _label :!via `Reverse`))

(event `self.ReceiveBeginPlay`
  (`KismetSystemLibrary.Delay` 3.0)
  (`self.FadeOut`)
  (`KismetSystemLibrary.Delay` 7.0)
  (`self.FadeIn`))

(fn `ResetMaterials`
  (for (_ _array_index) (`self.OriginalMaterials`)
    (`PrimitiveComponent.SetMaterial` (`self.Mesh`) _array_index null)))

(fn `SetMaterialsToDynamicInstances`
  (for (_array_element _array_index) (`self.DynamicMaterialInstances`)
    (`PrimitiveComponent.SetMaterial` (`self.Mesh`) _array_index _array_element)))

(fn `UserConstructionScript`
  (set `self.OriginalCursorVisResponse` (`PrimitiveComponent.GetCollisionResponseToChannel` (`self.Mesh`) "ECC_GameTraceChannel2"))
  (`KismetArrayLibrary.Array_Clear` (`self.DynamicMaterialInstances`))
  (set `self.OriginalMaterials` (`MeshComponent.GetMaterials` (`self.Mesh`)))
  (for _array_element (`self.FadeMaterialInstances`)
    (bind _returnvalue (`KismetMaterialLibrary.CreateDynamicMaterialInstance` _array_element))
    (`KismetArrayLibrary.Array_AddUnique` (`self.DynamicMaterialInstances`) _returnvalue)))