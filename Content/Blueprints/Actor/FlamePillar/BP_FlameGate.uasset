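; BP_FlameGate is a flame gate actor that ignites once when an actor tagged Player enters its trigger box.
; The overlap shows two lights, activates two Niagara effects, disables the box collision and plays an ignition timeline.
; When ignition finishes, the lights flicker endlessly by randomly chaining two timelines, each picking the next on completion.
; All timelines drive both lights through ScaleFlameIntensity, which multiplies the curve value by BaseIntensity.
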(event `ChooseTimeline`
  (switch `int` (`KismetMathLibrary.RandomIntegerInRange` 0 1)
    (:`Default`
      (`self.StartTimeLine_1` :!label _label))
    (:`0`
      (`self.StartTimeLine_0`))
    (:`1`
      (goto _label))))

(event `StartTimeLine_1`
  (bind (_direction _flameintensity) (`Timeline|Timeline_0` :!via `PlayFromStart`)
    (:`Update`
      (`self.ScaleFlameIntensity` _flameintensity))
    (:`Finished`
      (`self.ChooseTimeline`))))

(event `self.ReceiveBeginPlay`)

(event `StartTimeLine_0`
  (bind (_direction _flameintensity) (`Timeline|Timeline` :!via `PlayFromStart`)
    (:`Update`
      (`self.ScaleFlameIntensity` _flameintensity))
    (:`Finished`
      (`self.ChooseTimeline`))))

(event `self.Box.OnComponentBeginOverlap`
  (params (OverlappedComponent :type "PrimitiveComponent Object Reference") (OtherActor :type "Actor Object Reference") (OtherComp :type "PrimitiveComponent Object Reference") (OtherBodyIndex :type Integer) (bFromSweep :type Boolean) (SweepResult :type "HitResult Structure (by ref)"))
  (if (`self.ActorHasTag` OtherActor "Player")
    (`self.FlameOn`)
    (`SceneComponent.SetVisibility` (`self.Light`) true false)
    (`SceneComponent.SetVisibility` (`self.Light_1`) true false)
    (`ActorComponent.Activate` (`self.Niagara`) false)
    (`ActorComponent.Activate` (`self.Niagara_1`) false)
    (`PrimitiveComponent.SetCollisionEnabled` (`self.Box`) "NoCollision")))

(event `FlameOn`
  (bind (_direction _intensity) (`Timeline|FlameActivate` :!via `PlayFromStart`)
    (:`Update`
      (`self.ScaleFlameIntensity` _intensity))
    (:`Finished`
      (`self.ChooseTimeline`))))

(fn `ScaleFlameIntensity`
  (params (Scale :type "Float (double-precision)"))
  (`LightComponent.SetIntensity` (`self.Light`) (* Scale (`self.BaseIntensity`)))
  (`LightComponent.SetIntensity` (`self.Light_1`) (* Scale (`self.BaseIntensity`))))

(fn `UserConstructionScript`)