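; BP_FlamePillar is a flame pillar actor that flickers its light to suggest fire.
; From BeginPlay, it randomly picks one of two flame intensity timelines and plays it from the start.
; Each update scales the light's base intensity by the timeline value, and each finish triggers a new random pick, producing an endless, varied flicker without Tick.
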(event `ChooseTimeline`
  (switch `int` (`KismetMathLibrary.RandomIntegerInRange` 0 1)
    (:`Default`
      (`self.StartTimeLine_1` :!label _label))
    (:`0`
      (`self.StartTimeLine_0`))
    (:`1`
      (goto _label))))

(event `self.ReceiveBeginPlay`
  (`self.ChooseTimeline`))

(event `StartTimeLine_1`
  (bind (_direction _flameintensity) (`Timeline|FlameIntensity_1` :!via `PlayFromStart`)
    (:`Update`
      (`self.ScaleFlameIntensity` _flameintensity))
    (:`Finished`
      (`self.ChooseTimeline`))))

(event `StartTimeLine_0`
  (bind (_direction _flameintensity) (`Timeline|FlameIntensity_0` :!via `PlayFromStart`)
    (:`Update`
      (`self.ScaleFlameIntensity` _flameintensity))
    (:`Finished`
      (`self.ChooseTimeline`))))

(fn `ScaleFlameIntensity`
  (params (Scale :type "Float (double-precision)"))
  (`LightComponent.SetIntensity` (`self.Light`) (* Scale (`self.BaseIntensity`))))

(fn `UserConstructionScript`)