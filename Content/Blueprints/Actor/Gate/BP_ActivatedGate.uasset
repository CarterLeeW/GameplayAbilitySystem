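; BP_ActivatedGate is a two-leaf gate that swings open when its Open event is triggered and has no animated close.
; Open sets the Open flag once, then a timeline lerps PivotR and PivotL from zero rotation to their open rotations.
; LoadActor snaps both pivots to the open or closed pose from that flag, restoring state without animation.
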(event `self.ReceiveBeginPlay`)

(event `SaveObjectInterface.LoadActor`
  (if (`self.bOpen`)
    (`self.OpenPosition`)
    (else
      (`self.ClosePosition`))))

(event `Open`
  ;[1 1 1] We don't want to respond to this if the gate is already open
  (if (not (`self.bOpen`))
    (set `self.bOpen` true)
    (bind (_direction _lerpalpha) (`Timeline|OpenTimeline`)
      (:`Update`
        (`SceneComponent.K2_SetRelativeRotation` (`self.Pivot_R`) (`KismetMathLibrary.RLerp` (struct) (`self.OpenRotation_R`) _lerpalpha) false false)
        (`SceneComponent.K2_SetRelativeRotation` (`self.Pivot_L`) (`KismetMathLibrary.RLerp` (struct) (`self.OpenRotation_L`) _lerpalpha) false false)))))

(fn `ClosePosition`
  (`SceneComponent.K2_SetRelativeRotation` :`self` (`self.Pivot_R`) :`bTeleport` true)
  (`SceneComponent.K2_SetRelativeRotation` :`self` (`self.Pivot_L`) :`bTeleport` true))

(fn `OpenPosition`
  (`SceneComponent.K2_SetRelativeRotation` (`self.Pivot_R`) (`self.OpenRotation_R`) false true)
  (`SceneComponent.K2_SetRelativeRotation` (`self.Pivot_L`) (`self.OpenRotation_L`) false true))

(fn `UserConstructionScript`)