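; BP_MapEntrance_Stair is a stair map entrance that lights up a point light when highlighted.
; It stores the light's base intensity on BeginPlay and starts it at zero.
; Highlighting plays the LightOnOffSlider timeline, which scales that base intensity by its IntensityMultiplier track, and unhighlighting reverses the timeline.
; Highlight, begin-play and construction logic all call through to the parent class.
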(event `self.ReceiveBeginPlay`
  (`parent.ReceiveBeginPlay`)
  (set `self.LightIntensityBase` (`LightComponentBase.Intensity` (`self.PointLight`)))
  (`LightComponent.SetIntensity` (`self.PointLight`) 0.0))

(event `HighlightInterface.HighlightActor`
  (`parent.HighlightActor`)
  (bind (_direction _intensitymultiplier) (`Timeline|LightOnOffSlider` :!label _label)
    (:`Update`
      (`LightComponent.SetIntensity` (`self.PointLight`) (* (`self.LightIntensityBase`) _intensitymultiplier)))))

(event `HighlightInterface.UnHighlightActor`
  (`parent.UnHighlightActor`)
  (goto _label :!via `Reverse`))

(fn `UserConstructionScript`
  (`parent.UserConstructionScript`))