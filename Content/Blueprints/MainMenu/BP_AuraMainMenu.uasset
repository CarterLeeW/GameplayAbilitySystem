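; BP_AuraMainMenu is the main menu actor that bobs a fireball and brings up the menu.
; On BeginPlay it plays the menu music, adds WBP_MainMenu to the viewport, and switches to UI-only input with the cursor shown.
; A timeline offsets the FireBall's Z from its starting position, alternating forward and reverse playback through the GoUp flag for an endless hover loop.
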(event `Up`
  (bind (_direction _movement) (`Timeline|Timeline` :!via `PlayFromStart` :!label _label)
    (:`Update`
      (`self.UpdateFireBallLocation` _movement))
    (:`Finished`
      (if (`self.GoUp`)
        (`self.Down`)
        (set `self.GoUp` false)
        (else
          (`self.Up`)
          (set `self.GoUp` true))))))

(event `Down`
  (goto _label :!via `ReverseFromEnd`))

(event `self.ReceiveBeginPlay`
  (bind _returnvalue (`GameplayStatics.GetPlayerController` 0))
  (set `self.BasePosition` (`SceneComponent.K2_GetComponentLocation` (`self.FireBall`)))
  (`self.Up`)
  (set `self.GoUp` true)
  (`GameplayStatics.PlaySound2D` "/Game/Assets/Sounds/Music/Music_MainMenu.Music_MainMenu" 1.0 1.0 0.0 null null)
  (bind _returnvalue_2 (`|CreateWidget` "/Game/Blueprints/MainMenu/WBP_MainMenu.WBP_MainMenu_C"))
  (`UserWidget.AddToViewport` _returnvalue_2 0)
  (`WidgetBlueprintLibrary.SetInputMode_UIOnlyEx` _returnvalue _returnvalue_2)
  (set `PlayerController.bShowMouseCursor` true _returnvalue))

(fn `UpdateFireBallLocation`
  (params (In :type "Float (double-precision)"))
  (`SceneComponent.K2_SetWorldLocation` (`self.FireBall`) (`KismetMathLibrary.MakeVector` (.x (`self.BasePosition`)) (.y (`self.BasePosition`)) (+ (.z (`self.BasePosition`)) (* In 15.0))) false false))

(fn `UserConstructionScript`)